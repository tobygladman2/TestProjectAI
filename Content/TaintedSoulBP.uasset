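; TaintedSoulBP is a soul actor that trails behind the player after being touched.
; On overlap it stores the pawn as its follow target, increments the third-person character's souls count, saves the previous count and starts following.
; Each tick, only while the player's souls array is empty, it interpolates toward a point behind the target's forward vector at a configurable follow speed.
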(event EventBeginPlay)

(event EventTick
  (params (DeltaSeconds :type Float%20%28single-precision%29))
  (bind _followingtarget (Variables|Default|GetFollowingTarget))
  (bind _returnvalue (Class|TestProjectAICharacter|ReturnSoulsArray (Variables|Default|GetPlayer)))
  (if (== (Utilities|Array|Length _returnvalue) 0)
    (if (Variables|Default|GetisFollowing)
      (Transformation|SetActorLocation (Math|Interpolation|VInterpTo (Transformation|GetActorLocation) (+ (Transformation|GetActorLocation _followingtarget) (* (Transformation|GetActorForwardVector _followingtarget) "-150.000000,-150.000000,-150.000000")) DeltaSeconds (Variables|Default|GetSoulFollowSpeed)) false false))))

(event Collision|EventActorBeginOverlap
  (params (OtherActor :type Actor%20Object%20Reference))
  (bind _aspawn (Utilities|Casting|CastToPawn OtherActor))
  (Variables|Default|SetFollowingTarget _aspawn)
  (bind _asbp_third_person_character (Utilities|Casting|CastToBP_ThirdPersonCharacter OtherActor))
  (bind _output_get (Variables|Default|SetPlayer _asbp_third_person_character))
  (bind _returnvalue (Class|TestProjectAICharacter|GetSoulsCount _output_get))
  (Class|TestProjectAICharacter|SetSoulsCount _asbp_third_person_character (+ _returnvalue 1))
  (Variables|Default|SetcurrentSoulNumber _returnvalue)
  (Variables|Default|SetisFollowing true))

(fn ConstructionScript)